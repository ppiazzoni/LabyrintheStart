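; Door actor that slides vertically open and closed, tagged "Door" and color-coded along with its lock.
; The FOpentheDoor event plays a timeline, with play rate set from the inverse of TLOpenRate, that lerps the door mesh's relative Z toward FinalLocation.
; CloseDoor reverses the same timeline.
; The construction script sets the tag and creates one colored dynamic material shared by the door and lock meshes.
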(event Custom|CloseDoor
  (bind _alpha (Timeline|Timeline Reverse)
    (:Update
      (Transformation|SetRelativeLocation (Variables|Default|GetSM_Door) (Math|Vector|Lerp(Vector) "0, 0, 0" (Math|Vector|MakeVector 0.0 0.0 (Variables|Default|GetFinalLocation)) _alpha) false false))))

(event EventFOpentheDoor
  (Components|Timeline|SetPlayRate (Variables|Default|GetTimeline) (/ 1.0 (Variables|Default|GetTL_Open_Rate)))
  (bind _alpha (Timeline|Timeline PlayFromStart)
    (:Update
      (Transformation|SetRelativeLocation (Variables|Default|GetSM_Door) (Math|Vector|Lerp(Vector) "0, 0, 0" (Math|Vector|MakeVector 0.0 0.0 (Variables|Default|GetFinalLocation)) _alpha) false false))))

(fn ConstructionScript
  (Utilities|Array|Clear (Variables|Actor|GetTags))
  (Utilities|Array|AddUnique (Variables|Actor|GetTags) "Door")
  (bind _returnvalue (Rendering|Material|CreateDynamicMaterialInstance (Variables|Default|GetSM_Door) 0 "/Game/Blueprints/Materials/M_Basic_Parameters.M_Basic_Parameters" "None" :!class /Script/Engine.PrimitiveComponent))
  (bind _output_get (Variables|Default|SetDynMat_TriggerDoor _returnvalue))
  (Rendering|Material|SetVectorParameterValue _output_get "Color" (Variables|Default|GetColor) :!class /Script/Engine.MaterialInstanceDynamic)
  (Rendering|Material|SetMaterial (Variables|Default|GetSM_Lock) 0 (Variables|Default|GetDynMat_TriggerDoor)))