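; Trigger actor that opens a referenced door the first time anything overlaps its box, then turns its base dark grey.
; DoOnce limits it to one activation, and a Blueprint Interface message reaches the door without a cast dependency.
; The construction script tags the actor "DoorTrigger" and creates the base's dynamic material, tinted by the Color variable.
; Unconnected player-tag and cast nodes remain as annotated alternatives.
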(event OnComponentBeginOverlap(Box)
  (params (OverlappedComponent :type Primitive%20Component%20Object%20Reference) (OtherActor :type Actor%20Object%20Reference) (OtherComp :type Primitive%20Component%20Object%20Reference) (OtherBodyIndex :type Integer) (bFromSweep :type Boolean) (SweepResult :type Hit%20Result%20Structure%20%28by%20ref%29))
  (Utilities|FlowControl|DoOnce false :!pinned true ; Do the Logic JUST one time
    (:Completed
      ;[0 1 0] Better to use a BP Interface
      (Class|BPITriggers|FOpentheDoor(Message) (Variables|Default|GetDoorREF))
      (Rendering|Material|SetVectorParameterValue (Variables|Default|GetDynMat_TriggerBase) "Color" "(R=0.250000,G=0.250000,B=0.250000,A=1.000000)" :!class /Script/Engine.MaterialInstanceDynamic))))

(fn ConstructionScript
  (Utilities|Array|Clear (Variables|Actor|GetTags))
  (Utilities|Array|AddUnique (Variables|Actor|GetTags) "DoorTrigger")
  (bind _returnvalue (Rendering|Material|CreateDynamicMaterialInstance (Variables|Default|GetBase) 0 "/Game/Blueprints/Materials/M_Basic_Parameters.M_Basic_Parameters" "None" :!class /Script/Engine.PrimitiveComponent))
  (bind _output_get (Variables|Default|SetDynMat_TriggerBase _returnvalue))
  (Rendering|Material|SetVectorParameterValue _output_get "Color" (Variables|Default|GetColor) :!class /Script/Engine.MaterialInstanceDynamic))