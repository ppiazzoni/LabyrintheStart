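; Teleporter pad that moves the overlapping actor to a linked TeleportREF, matching its rotation and setting player 0's control rotation.
; On overlap it messages the destination to block itself, preventing bounce-back, then teleports through a DoOnce that resets after a delay.
; End overlap re-enables the pad after ReActivationDelay.
; A dynamic material built in construction shows its Color when active, grey when blocked, cooling down or unlinked.
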(event OnComponentBeginOverlap(Box)
  (params (OverlappedComponent :type Primitive%20Component%20Object%20Reference) (OtherActor :type Actor%20Object%20Reference) (OtherComp :type Primitive%20Component%20Object%20Reference) (OtherBodyIndex :type Integer) (bFromSweep :type Boolean) (SweepResult :type Hit%20Result%20Structure%20%28by%20ref%29))
  (Variables|Default|SetOther%20Actor OtherActor)
  (Utilities|IsValid (Variables|Default|GetTeleportREF)
    (:Is%20Valid
      (Class|BPITriggers|FBlockReftoTeleport(Message) (Variables|Default|GetTeleportREF))
      (if (Variables|Default|GetCanTeleport?)
        (Utilities|FlowControl|DoOnce false :!pinned true ; Do the Logic JUST one time
          (:Completed
            (Rendering|Material|SetVectorParameterValue (Variables|Default|GetDynMat_TriggerBase) "Color" "(R=0.250000,G=0.250000,B=0.250000,A=1.000000)" :!class /Script/Engine.MaterialInstanceDynamic)
            (Transformation|SetActorLocationAndRotation (Variables|Default|GetOther%20Actor) (+ (Transformation|GetActorLocation (Variables|Default|GetTeleportREF)) "0.000000,0.000000,10.000000") (Transformation|GetActorRotation (Variables|Default|GetTeleportREF)))
            (Pawn|SetControlRotation (Game|GetPlayerController 0) (Transformation|GetActorRotation (Variables|Default|GetTeleportREF)))
            (Utilities|FlowControl|Delay 3.0)
            (Rendering|Material|SetVectorParameterValue (Variables|Default|GetDynMat_TriggerBase) "Color" (Variables|Default|GetColor) :!class /Script/Engine.MaterialInstanceDynamic)
            (CallFunction|RDOTeleport)))))))

(event OnComponentEndOverlap(Box)
  (params (OverlappedComponent :type Primitive%20Component%20Object%20Reference) (OtherActor :type Actor%20Object%20Reference) (OtherComp :type Primitive%20Component%20Object%20Reference) (OtherBodyIndex :type Integer))
  (Utilities|IsValid (Variables|Default|GetTeleportREF)
    (:Is%20Valid
      (Utilities|FlowControl|Delay (Variables|Default|GetReActivationDelay))
      (Rendering|Material|SetVectorParameterValue (Variables|Default|GetDynMat_TriggerBase) "Color" (Variables|Default|GetColor) :!class /Script/Engine.MaterialInstanceDynamic)
      (Variables|Default|SetCanTeleport? true))))

(event Custom|RDO_Teleport
  (Utilities|FlowControl|DoOnce false) ; enters at Reset
)

(event EventFBlockReftoTeleport
  (Rendering|Material|SetVectorParameterValue (Variables|Default|GetDynMat_TriggerBase) "Color" "(R=0.250000,G=0.250000,B=0.250000,A=1.000000)" :!class /Script/Engine.MaterialInstanceDynamic)
  (Variables|Default|SetCanTeleport? false))

(fn ConstructionScript
  (Utilities|Array|Clear (Variables|Actor|GetTags))
  (Utilities|Array|AddUnique (Variables|Actor|GetTags) "Teleport")
  (bind _returnvalue (Rendering|Material|CreateDynamicMaterialInstance (Variables|Default|GetBase) 0 "/Game/Blueprints/Materials/M_Basic_Parameters.M_Basic_Parameters" "None" :!class /Script/Engine.PrimitiveComponent))
  (bind _output_get (Variables|Default|SetDynMat_TriggerBase _returnvalue))
  (Rendering|Material|SetVectorParameterValue _output_get "Color" (Variables|Default|GetColor) :!class /Script/Engine.MaterialInstanceDynamic)
  (Rendering|Material|SetMaterial (Variables|Default|GetBase1) 0 (Variables|Default|GetDynMat_TriggerBase))
  (Utilities|IsValid (Variables|Default|GetTeleportREF)
    (:Is%20Not%20Valid
      (Rendering|Material|SetVectorParameterValue (Variables|Default|GetDynMat_TriggerBase) "Color" "(R=0.250000,G=0.250000,B=0.250000,A=1.000000)" :!class /Script/Engine.MaterialInstanceDynamic))))