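; Laser trap actor that spans a capsule between two laser bases, LaserA and LaserB, and tags itself "LaserTrap".
; The construction script moves LaserB to a configurable location, then centers, aligns and sizes the capsule from the offset between the two bases, with an adjustable radius.
; Both spheres share one dynamic material instance set to the safe emissive color, while the charge color is stored in Color.
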(fn ConstructionScript
  (bind _laser_a (Variables|Default|GetLaser_A))
  (bind _laser_b (Variables|Default|GetLaser_B))
  (bind _relativelocation (Variables|/Script/Engine.SceneComponent|GetRelativeLocation _laser_b))
  (bind _relativelocation_2 (Variables|/Script/Engine.SceneComponent|GetRelativeLocation _laser_a))
  (Utilities|Array|Clear (Variables|Actor|GetTags))
  (Utilities|Array|AddUnique (Variables|Actor|GetTags) "LaserTrap")
  (Utilities|FlowControl|Sequence
    (:then_0
      (Transformation|SetRelativeLocation (Variables|Default|GetLaser_B) (Variables|Default|GetLaserBase_B_Location) false false)
      (bind _output_get (LocalVariables|SetL_MidDistance (/ (- _relativelocation _relativelocation_2) 2.0)))
      (Transformation|SetRelativeLocationAndRotation (Variables|Default|GetCapsule) _output_get (Math|Rotator|CombineRotators "90.000000,0.000000,0.000000" (Math|Rotator|FindLookatRotation _relativelocation _relativelocation_2)) false false)
      (Components|Capsule|SetCapsuleHalfHeight (Variables|Default|GetCapsule) (Math|Vector|VectorLength (LocalVariables|GetL_MidDistance)) true)
      (Components|Capsule|SetCapsuleRadius (Variables|Default|GetCapsule) (Variables|Default|GetCapsuleRadius) true))
    (:then_1
      (bind _returnvalue (Rendering|Material|CreateDynamicMaterialInstance (Variables|Default|GetSphere_B) 0 "/Game/Blueprints/Materials/M_Basic_Parameters.M_Basic_Parameters" "None" :!class /Script/Engine.PrimitiveComponent))
      (bind _output_get_2 (Variables|Default|SetDynMat_Spheres _returnvalue))
      (Rendering|Material|SetMaterial (Variables|Default|GetSphere_A) 0 _output_get_2)
      (Rendering|Material|SetVectorParameterValue (Variables|Default|GetDynMat_Spheres) "EmissiveColor" (Variables|Default|GetSafeColor) :!class /Script/Engine.MaterialInstanceDynamic)
      (Variables|Default|SetColor (Variables|Default|GetChargeColor)))))