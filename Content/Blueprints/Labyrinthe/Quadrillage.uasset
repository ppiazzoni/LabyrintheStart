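; Quadrillage is a grid actor for the labyrinth that lays out cell meshes as instances of a hierarchical instanced static mesh.
; Its construction script reads mesh, row and column counts and cell size from a Structure variable, then adds evenly spaced instances in nested loops.
; The column loop runs up to the column count without the minus one used for rows.
; Event handlers are empty, and older grid, random-scale and list code is disconnected.
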(event Collision|EventActorBeginOverlap
  (params (OtherActor :type Actor%20Object%20Reference)))

(event EventTick
  (params (DeltaSeconds :type Float%20%28single-precision%29)))

(event EventBeginPlay)

(fn ConstructionScript
  (bind _structure (Variables|Default|GetStructure))
  (Components|StaticMesh|SetStaticMesh (Variables|Default|GetHISM) (.meshcase _structure))
  (for _index (range 0 (- (.ligne _structure) 1))
    (bind _output_get (Variables|Default|SetPositionX (Math|Vector|MakeVector (* _index (.taille _structure)) 0.0 0.0)))
    (for _index_2 (range 0 (.colonne _structure))
      (bind _output_get_2 (Variables|Default|SetPositionY (Math|Vector|MakeVector 0.0 (* _index_2 (.taille _structure)) 0.0)))
      (Components|InstancedStaticMesh|AddInstance (Variables|Default|GetHISM) (Math|Transform|MakeTransform (+ _output_get_2 _output_get) "0, 0, 0" "1.000000,1.000000,1.000000") false))))