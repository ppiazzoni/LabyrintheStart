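; BP_Chain builds a decorative chain along a spline in the construction script, with no active gameplay logic.
; It clears the instanced static mesh component and adds link instances at fixed intervals, aligned to the spline.
; Every other link is rotated 90 degrees so the links appear interlocked.
; Separate start and end meshes are snapped to the two ends of the spline.
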(event EventBeginPlay)

(event Collision|EventActorBeginOverlap
  (params (OtherActor :type Actor%20Object%20Reference)))

(event EventTick
  (params (DeltaSeconds :type Float%20%28single-precision%29)))

(fn ConstructionScript
  (bind _spline (Variables|Default|GetSpline))
  (bind _returnvalue (Spline|GetSplineLength _spline))
  (Components|InstancedStaticMesh|ClearInstances (Variables|Default|GetHISM_00))
  (Components|StaticMesh|SetStaticMesh (Variables|Default|GetHISM_00) (Variables|Default|GetSM_ChainLink))
  (for _index (range 0 (Math|Float|Floor (/ (Spline|GetSplineLength (Variables|Default|GetSpline)) (Math|Float|MakeLiteralFloat 5e+01))))
    (bind _output_get (LocalVariables|SetL_Index _index))
    (if (not (> _output_get 0))
      (Transformation|SetRelativeLocationAndRotation (Variables|Default|GetSM_ChainStart) (Spline|GetLocationatDistanceAlongSpline (Variables|Default|GetSpline) 0.0 "Local") (Spline|GetRotationatDistanceAlongSpline (Variables|Default|GetSpline) 0.0 "Local") false false)
      (else
        (Components|InstancedStaticMesh|AddInstance (Variables|Default|GetHISM_00) (Math|Transform|MakeTransform (Spline|GetLocationatDistanceAlongSpline (Variables|Default|GetSpline) (* _index 5e+01) "Local") (Math|Rotator|CombineRotators (select (!= (Math|Integer|%(Integer) (LocalVariables|GetL_Index) 2) 0) "0.000000,0.000000,90.000000" "0, 0, 0") (Spline|GetRotationatDistanceAlongSpline (Variables|Default|GetSpline) (* _index 5e+01) "Local"))) false))))
  (Transformation|SetRelativeLocationAndRotation (Variables|Default|GetSM_ChainEnd) (Spline|GetLocationatDistanceAlongSpline (Variables|Default|GetSpline) _returnvalue "Local") (Spline|GetRotationatDistanceAlongSpline (Variables|Default|GetSpline) _returnvalue "Local") false false))