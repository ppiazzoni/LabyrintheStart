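; BP_StoneSpline_00 is a spline placement tool that lays out stone meshes along a path.
; The construction script rebuilds a hierarchical instanced static mesh, spacing the set stone count evenly from end to end, aligned to the spline with a Z offset.
; An optional debug display toggles name and count text renders, and a zero count prints a warning.
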(fn ConstructionScript
  (Components|InstancedStaticMesh|ClearInstances (Variables|Default|GetHISM_00))
  (Components|StaticMesh|SetStaticMesh (Variables|Default|GetHISM_00) (Variables|Default|GetSM_Stone))
  (if (> (Variables|Default|GetStones) 0)
    (for _index (range 0 (- (Variables|Default|GetStones) 1))
      (LocalVariables|SetL_StoneXLocation (+ (Spline|GetLocationatDistanceAlongSpline (Variables|Default|GetSpline) (* _index (/ (Spline|GetSplineLength (Variables|Default|GetSpline)) (- (Variables|Default|GetStones) 1))) "Local") (Math|Vector|MakeVector 0.0 0.0 (Variables|Default|GetStoneZOffset))))
      (LocalVariables|SetL_StoneXRotation (Spline|GetRotationatDistanceAlongSpline (Variables|Default|GetSpline) (* _index (/ (Spline|GetSplineLength (Variables|Default|GetSpline)) (- (Variables|Default|GetStones) 1))) "Local"))
      (LocalVariables|SetL_InstanceTransform (Math|Transform|MakeTransform (LocalVariables|GetL_StoneXLocation) (LocalVariables|GetL_StoneXRotation) (LocalVariables|GetL_StoneScale)))
      (Components|InstancedStaticMesh|AddInstance (Variables|Default|GetHISM_00) (LocalVariables|GetL_InstanceTransform) false))
    (else
      (Development|PrintString "No Stones!!" true true "(R=1.000000,G=1.000000,B=1.000000,A=1.000000)" 3.0)))
  (Rendering|SetVisibility (Variables|Default|GetCubeCount) (Variables|Default|GetRenderText_?) false)
  (Rendering|SetVisibility (Variables|Default|GetBp_Name) (Variables|Default|GetRenderText_?) false)
  ;[1 1 0 0.15] Debug Only
  (if (Variables|Default|GetRenderText_?)
    (Rendering|Components|TextRender|SetText (Variables|Default|GetCubeCount) (Utilities|Text|ToText(String) (Utilities|String|Append "Cube Count : " (Utilities|String|ToString(Integer) (Components|InstancedStaticMesh|GetInstanceCount (Variables|Default|GetHISM_00))))))))