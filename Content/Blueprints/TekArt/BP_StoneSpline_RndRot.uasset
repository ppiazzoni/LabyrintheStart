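; BP_StoneSpline_RndRot is a construction-script placement tool that lines a spline with randomly rotated stone meshes, tagged as Wall_Spline.
; It rebuilds one HISM component, spacing the stone count evenly along the spline with a Z offset.
; A seeded random stream varies each stone's rotation, relative to the spline direction, and its per-axis scale, keeping layouts repeatable.
; Optional debug text components show the instance count and Blueprint name.
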(fn ConstructionScript
  (Utilities|Array|Clear (Variables|Actor|GetTags))
  (Utilities|Array|AddUnique (Variables|Actor|GetTags) "Wall_Spline")
  (Variables|Default|SetStream (Math|Random|MakeRandomStream (Variables|Default|GetStream%20Initial%20Seed)))
  (Components|InstancedStaticMesh|ClearInstances (Variables|Default|GetHISM_00))
  (Components|StaticMesh|SetStaticMesh (Variables|Default|GetHISM_00) (Variables|Default|GetSM_Stone))
  (if (> (Variables|Default|GetStones) 0)
    (for _index (range 0 (- (Variables|Default|GetStones) 1))
      (LocalVariables|SetL_StoneXLocation (+ (Spline|GetLocationatDistanceAlongSpline (Variables|Default|GetSpline) (* _index (/ (Spline|GetSplineLength (Variables|Default|GetSpline)) (- (Variables|Default|GetStones) 1))) "Local") (Math|Vector|MakeVector 0.0 0.0 (Variables|Default|GetStoneZOffset))))
      (LocalVariables|SetL_StoneXRotation (Math|Rotator|CombineRotators (Spline|GetRotationatDistanceAlongSpline (Variables|Default|GetSpline) (* _index (/ (Spline|GetSplineLength (Variables|Default|GetSpline)) (- (Variables|Default|GetStones) 1))) "Local") (Class|KismetMathLibrary|RandomRotatorfromStream (Variables|Default|GetStream) true)))
      (Components|InstancedStaticMesh|AddInstance (Variables|Default|GetHISM_00) (Math|Transform|MakeTransform (LocalVariables|GetL_StoneXLocation) (LocalVariables|GetL_StoneXRotation) (Math|Vector|MakeVector (Math|Random|RandomFloatinRangefromStream (Variables|Default|GetStream) (Variables|Default|GetMinScale) (Variables|Default|GetMaxScale)) (Math|Random|RandomFloatinRangefromStream (Variables|Default|GetStream) (Variables|Default|GetMinScale) (Variables|Default|GetMaxScale)) (Math|Random|RandomFloatinRangefromStream (Variables|Default|GetStream) (Variables|Default|GetMinScale) (Variables|Default|GetMaxScale)))) false))
    (Rendering|SetVisibility (Variables|Default|GetCubeCount) (Variables|Default|GetRenderText_?) false)
    (Rendering|SetVisibility (Variables|Default|GetBp_Name) (Variables|Default|GetRenderText_?) false)
    ;[1 1 0 0.15] Debug Only
    (if (Variables|Default|GetRenderText_?)
      (Rendering|Components|TextRender|SetText (Variables|Default|GetCubeCount) (Utilities|Text|ToText(String) (Utilities|String|Append "Cube Count : " (Utilities|String|ToString(Integer) (Components|InstancedStaticMesh|GetInstanceCount (Variables|Default|GetHISM_00)))))))))