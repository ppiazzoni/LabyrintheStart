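; Editor tool actor that converts all static mesh actors sharing a chosen tag into hierarchical instanced meshes.
; The construction script hides tagged actors, disables their collision, and builds one HISM per unique mesh, adding instances at their transforms.
; ReleaseThem clears the instances and restores the original actors; it also runs before each rebuild.
; Text labels show tag and actor count, while a sphere turns red when converted, green when released.
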(event Custom|Release%20Them
  ;[1 1 1] Release Instances
  ; UnHide Elements
  ; Call in Editor
  (for _array_element (Variables|Default|GetArray_ActorsToConvert)
    (Rendering|SetVisibility (Variables|/Script/Engine.StaticMeshActor|GetStaticMeshComponent _array_element) true false)
    (Collision|SetCollisionEnabled (Variables|/Script/Engine.StaticMeshActor|GetStaticMeshComponent _array_element) "QueryAndPhysics"))
  (Rendering|Components|TextRender|SetText (Variables|Default|GetRT_Elements) (Utilities|Text|MakeLiteralText "Released!!"))
  (Rendering|Components|TextRender|SetText (Variables|Default|GetRT_Elements) (Utilities|Text|MakeLiteralText "Actors : 0"))
  (Utilities|Array|Clear (Variables|Default|GetArray_ActorsToConvert))
  (Utilities|Array|Clear (Variables|Default|GetArray_ActorTransform))
  (Utilities|Array|Clear (Variables|Default|GetArray_UniqueSMs))
  (Utilities|Array|Clear (Variables|Default|GetActorsIDList))
  (for _array_element_2 (Variables|Default|GetArray_HISMComponent)
    (Components|InstancedStaticMesh|ClearInstances _array_element_2)
    (Components|DestroyComponent _array_element_2))
  (Utilities|Array|Clear (Variables|Default|GetArray_HISMComponent))
  (Rendering|Material|SetVectorParameterValue (Variables|Default|GetDynMatREF) "Color" "(R=0.000000,G=1.000000,B=0.000000,A=1.000000)" :!class /Script/Engine.MaterialInstanceDynamic))

(fn ConstructionScript
  (Utilities|Array|Clear (Variables|Actor|GetTags))
  (Utilities|Array|AddUnique (Variables|Actor|GetTags) "BP_Platon")
  (Variables|Default|SetConvertToInstances false)
  (bind _returnvalue (Rendering|Material|CreateDynamicMaterialInstance (Variables|Default|GetSphere) 0 "/Game/Blueprints/Materials/M_Basic_Parameters.M_Basic_Parameters" "None" :!class /Script/Engine.PrimitiveComponent))
  (Variables|Default|SetDynMatREF _returnvalue)
  (Rendering|Material|SetVectorParameterValue (Variables|Default|GetDynMatREF) "Color" "(R=0.000000,G=1.000000,B=0.000000,A=1.000000)" :!class /Script/Engine.MaterialInstanceDynamic)
  (if (not (== (Variables|Default|GetTag) ""))
    (Rendering|Components|TextRender|SetText (Variables|Default|GetRT_Tag) (Utilities|Text|ToText(String) (Utilities|String|Append "Tag : " (Utilities|String|ToString(Name) (Variables|Default|GetTag)))))
    (Rendering|Components|TextRender|SetText (Variables|Default|GetRT_Elements) (Utilities|Text|ToText(String) (Utilities|String|Append "Actors : " (Utilities|String|ToString(Integer) (select (Utilities|Array|IsValidIndex (LocalVariables|GetL_Array_ActorsFound)) (Utilities|Array|Length (LocalVariables|GetL_Array_ActorsFound)) 0)))))
    (CallFunction|ReleaseThem)
    (bind _outactors (Actor|GetAllActorsOfClasswithTag "/Script/Engine.StaticMeshActor" (Variables|Default|GetTag)))
    (if (Utilities|Array|IsValidIndex _outactors)
      (Variables|Default|SetArray_ActorsToConvert _outactors)
      (Rendering|Components|TextRender|SetText (Variables|Default|GetRT_Elements) (Utilities|Text|ToText(String) (Utilities|String|Append "Actors : " (Utilities|String|ToString(Integer) (Utilities|Array|Length (Variables|Default|GetArray_ActorsToConvert))))))
      (for _array_element (Variables|Default|GetArray_ActorsToConvert)
        (Variables|Default|SetREF_ActorToConvert _array_element)
        (Rendering|SetVisibility (Variables|/Script/Engine.StaticMeshActor|GetStaticMeshComponent (Variables|Default|GetREF_ActorToConvert)) false false)
        (Collision|SetCollisionEnabled (Variables|/Script/Engine.StaticMeshActor|GetStaticMeshComponent (Variables|Default|GetREF_ActorToConvert)) "NoCollision")
        (Variables|Default|SetElement_StaticMesh (Variables|/Script/Engine.StaticMeshComponent|GetStaticMesh (Variables|/Script/Engine.StaticMeshActor|GetStaticMeshComponent (Variables|Default|GetREF_ActorToConvert))))
        (Variables|Default|SetElement_Transform (Transformation|GetActorTransform (Variables|Default|GetREF_ActorToConvert)))
        (if (== (Utilities|Array|FindItem (Variables|Default|GetArray_UniqueSMs) (Variables|Default|GetElement_StaticMesh)) -1)
          (bind _returnvalue_2 (Utilities|Array|AddUnique (Variables|Default|GetArray_UniqueSMs) (Variables|Default|GetElement_StaticMesh)))
          (Utilities|Array|Add (Variables|Default|GetActorsIDList) _returnvalue_2)
          (Utilities|Array|Add (Variables|Default|GetArray_ActorTransform) (Variables|Default|GetElement_Transform))
          (else
            (Utilities|Array|Add (Variables|Default|GetActorsIDList) (Utilities|Array|FindItem (Variables|Default|GetArray_UniqueSMs) (Variables|Default|GetElement_StaticMesh)))
            (Utilities|Array|Add (Variables|Default|GetArray_ActorTransform) (Variables|Default|GetElement_Transform)))))
      (for _array_element_2 (Variables|Default|GetArray_UniqueSMs)
        (bind _returnvalue_3 (AddComponent|AddHierarchicalInstancedStaticMeshComponent true))
        (Utilities|Array|Add (Variables|Default|GetArray_HISMComponent) _returnvalue_3))
      (for (_array_element_3 _array_index) (Variables|Default|GetActorsIDList)
        (Components|StaticMesh|SetStaticMesh (Utilities|Array|Get(acopy) (Variables|Default|GetArray_HISMComponent) _array_element_3) (Utilities|Array|Get(acopy) (Variables|Default|GetArray_UniqueSMs) _array_element_3))
        (Components|InstancedStaticMesh|AddInstance (Utilities|Array|Get(acopy) (Variables|Default|GetArray_HISMComponent) _array_element_3) (Utilities|Array|Get(acopy) (Variables|Default|GetArray_ActorTransform) _array_index) true))
      (Rendering|Material|SetVectorParameterValue (Variables|Default|GetDynMatREF) "Color" "(R=1.000000,G=0.000000,B=0.000000,A=1.000000)" :!class /Script/Engine.MaterialInstanceDynamic)
      (else
        (Rendering|Components|TextRender|SetText (Variables|Default|GetRT_Elements) (Utilities|Text|MakeLiteralText "No Actors Found!!"))
        (CallFunction|ReleaseThem)))
    (else
      (Rendering|Components|TextRender|SetText (Variables|Default|GetRT_Tag) (Utilities|Text|MakeLiteralText "No Tag Selected!!!"))
      (CallFunction|ReleaseThem))))