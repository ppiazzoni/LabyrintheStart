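; Editor tool actor that converts tagged StaticMeshActors into hierarchical instanced meshes.
; The construction script releases previous results, then hides matching actors and disables their collision.
; It builds one HISM component per unique mesh and slot-0 material pair, adding instances at original transforms.
; ReleaseThem restores the actors and destroys the HISMs, while text labels and a green/red sphere show status.
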(event Custom|Release%20Them
  ;[1 1 1] Release Instances
  ; UnHide Elements
  ; Call in Editor
  (for _array_element (Variables|Default|GetArray_ActorsToConvert)
    (Rendering|SetVisibility (Variables|/Script/Engine.StaticMeshActor|GetStaticMeshComponent _array_element) true false)
    (Collision|SetCollisionEnabled (Variables|/Script/Engine.StaticMeshActor|GetStaticMeshComponent _array_element) "QueryAndPhysics"))
  (Rendering|Components|TextRender|SetText (Variables|Default|GetElements%20:) (Utilities|Text|MakeLiteralText "Released!!"))
  (Rendering|Components|TextRender|SetText (Variables|Default|GetElements%20:) (Utilities|Text|MakeLiteralText "Actors : 0"))
  (Utilities|Array|Clear (Variables|Default|GetArray_ActorsToConvert))
  (Utilities|Array|Clear (Variables|Default|GetArray_Element_Transform))
  (Utilities|Array|Clear (Variables|Default|GetStruct_PlatonPairs))
  (Utilities|Array|Clear (Variables|Default|GetStruct_UniquePlatonPairs))
  (for _array_element_2 (Variables|Default|GetArray_HISMComponent)
    (Components|InstancedStaticMesh|ClearInstances _array_element_2)
    (Components|DestroyComponent _array_element_2))
  (Utilities|Array|Clear (Variables|Default|GetArray_HISMComponent)))

(fn ConstructionScript
  (Utilities|Array|Clear (Variables|Actor|GetTags))
  (Utilities|Array|AddUnique (Variables|Actor|GetTags) "BP_Platon")
  (Variables|Default|SetConvertToInstances false)
  (bind _returnvalue (Rendering|Material|CreateDynamicMaterialInstance (Variables|Default|GetSphere) 0 "/Game/Blueprints/Materials/M_Basic_Parameters.M_Basic_Parameters" "None" :!class /Script/Engine.PrimitiveComponent))
  (Variables|Default|SetDynMatREF _returnvalue)
  (Rendering|Material|SetVectorParameterValue (Variables|Default|GetDynMatREF) "Color" "(R=0.000000,G=1.000000,B=0.000000,A=1.000000)" :!class /Script/Engine.MaterialInstanceDynamic)
  (if (not (== (Variables|Default|GetTag) ""))
    (Rendering|Components|TextRender|SetText (Variables|Default|GetRT_Tag) (Utilities|Text|ToText(String) (Utilities|String|Append "Tag : " (Utilities|String|ToString(Name) (Variables|Default|GetTag)))))
    (Rendering|Components|TextRender|SetText (Variables|Default|GetElements%20:) (Utilities|Text|ToText(String) (Utilities|String|Append "Actors : " (Utilities|String|ToString(Integer) (select (Utilities|Array|IsValidIndex (LocalVariables|GetL_Array_ActorsFound)) (Utilities|Array|Length (LocalVariables|GetL_Array_ActorsFound)) 0)))))
    (CallFunction|ReleaseThem)
    (bind _outactors (Actor|GetAllActorsOfClasswithTag "/Script/Engine.StaticMeshActor" (Variables|Default|GetTag)))
    (if (Utilities|Array|IsValidIndex _outactors)
      (Variables|Default|SetArray_ActorsToConvert _outactors)
      (Rendering|Components|TextRender|SetText (Variables|Default|GetElements%20:) (Utilities|Text|ToText(String) (Utilities|String|Append "Actors : " (Utilities|String|ToString(Integer) (Utilities|Array|Length (Variables|Default|GetArray_ActorsToConvert))))))
      (for (_array_element _array_index) (Variables|Default|GetArray_ActorsToConvert)
        (Variables|Default|SetREF_ActorToConvert _array_element)
        (Variables|Default|SetActorsToConvert_Index _array_index)
        (Rendering|SetVisibility (Variables|/Script/Engine.StaticMeshActor|GetStaticMeshComponent (Variables|Default|GetREF_ActorToConvert)) false false)
        (Collision|SetCollisionEnabled (Variables|/Script/Engine.StaticMeshActor|GetStaticMeshComponent (Variables|Default|GetREF_ActorToConvert)) "NoCollision")
        (Variables|Default|SetElement_StaticMesh (Variables|/Script/Engine.StaticMeshComponent|GetStaticMesh (Variables|/Script/Engine.StaticMeshActor|GetStaticMeshComponent (Variables|Default|GetREF_ActorToConvert))))
        (Variables|Default|SetElement_Material (Rendering|Material|GetMaterial (Variables|/Script/Engine.StaticMeshActor|GetStaticMeshComponent (Variables|Default|GetREF_ActorToConvert)) 0))
        (Utilities|Array|Add (Variables|Default|GetArray_Element_Transform) (Transformation|GetActorTransform (Variables|Default|GetREF_ActorToConvert)))
        (Utilities|Array|Add (Variables|Default|GetStruct_PlatonPairs) (Utilities|Struct|MakeStruct_PlatonPairs (Utilities|Map|MakeMap (Variables|Default|GetElement_StaticMesh) (Variables|Default|GetElement_Material)) 0))
        (Utilities|Array|AddUnique (Variables|Default|GetStruct_UniquePlatonPairs) (Utilities|Struct|MakeStruct_PlatonPairs (Utilities|Map|MakeMap (Variables|Default|GetElement_StaticMesh) (Variables|Default|GetElement_Material)) 0)))
      (for _index (range 0 (- (Utilities|Array|Length (Variables|Default|GetStruct_UniquePlatonPairs)) 1))
        (bind _returnvalue_2 (AddComponent|AddHierarchicalInstancedStaticMeshComponent false (Transformation|GetActorTransform)))
        (Utilities|Array|Add (Variables|Default|GetArray_HISMComponent) _returnvalue_2))
      (for (_array_element_2 _array_index_2) (Variables|Default|GetArray_ActorsToConvert)
        (Rendering|Material|SetMaterial (Utilities|Array|Get(acopy) (Variables|Default|GetArray_HISMComponent) (Utilities|Array|FindItem (Variables|Default|GetStruct_UniquePlatonPairs) (Utilities|Array|Get(acopy) (Variables|Default|GetStruct_PlatonPairs) _array_index_2))) 0 (.Value (Utilities|Map|Find (.SM_MAT (Utilities|Struct|BreakStruct_PlatonPairs (Utilities|Array|Get(acopy) (Variables|Default|GetStruct_PlatonPairs) _array_index_2))) (Variables|/Script/Engine.StaticMeshComponent|GetStaticMesh (Variables|/Script/Engine.StaticMeshActor|GetStaticMeshComponent _array_element_2)))))
        (Components|StaticMesh|SetStaticMesh (Utilities|Array|Get(acopy) (Variables|Default|GetArray_HISMComponent) (Utilities|Array|FindItem (Variables|Default|GetStruct_UniquePlatonPairs) (Utilities|Array|Get(acopy) (Variables|Default|GetStruct_PlatonPairs) _array_index_2))) (Variables|/Script/Engine.StaticMeshComponent|GetStaticMesh (Variables|/Script/Engine.StaticMeshActor|GetStaticMeshComponent _array_element_2)))
        (Components|InstancedStaticMesh|AddInstance (Utilities|Array|Get(acopy) (Variables|Default|GetArray_HISMComponent) (Utilities|Array|FindItem (Variables|Default|GetStruct_UniquePlatonPairs) (Utilities|Array|Get(acopy) (Variables|Default|GetStruct_PlatonPairs) _array_index_2))) (Utilities|Array|Get(acopy) (Variables|Default|GetArray_Element_Transform) _array_index_2) true))
      (Rendering|Material|SetVectorParameterValue (Variables|Default|GetDynMatREF) "Color" "(R=1.000000,G=0.000000,B=0.000000,A=1.000000)" :!class /Script/Engine.MaterialInstanceDynamic)
      (else
        (Rendering|Components|TextRender|SetText (Variables|Default|GetElements%20:) (Utilities|Text|MakeLiteralText "No Actors Found!!"))))
    (else
      (Rendering|Components|TextRender|SetText (Variables|Default|GetRT_Tag) (Utilities|Text|MakeLiteralText "No Tag Selected!!!"))
      (CallFunction|ReleaseThem))))