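; Spline actor tagged Wall_Spline that lines a set number of stone meshes along its spline.
; The construction script rebuilds HISM instances at even distances, following spline rotation with a Z offset.
; Each instance gets RGB through per-instance custom data, taken from CustomColors or, for missing or zero entries, the dynamic material's BaseColor.
; An optional debug text displays the instance count.
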(fn ConstructionScript
  (Utilities|Array|Clear (Variables|Actor|GetTags))
  (Utilities|Array|AddUnique (Variables|Actor|GetTags) "Wall_Spline")
  (Components|InstancedStaticMesh|ClearInstances (Variables|Default|GetHISM_00))
  (Components|StaticMesh|SetStaticMesh (Variables|Default|GetHISM_00) (Variables|Default|GetSM_Stone))
  (bind _returnvalue (Rendering|Material|CreateDynamicMaterialInstance (Variables|Default|GetHISM_00) 0 (Variables|Default|GetMaterial) "None" :!class /Script/Engine.PrimitiveComponent))
  (bind _output_get (LocalVariables|SetL_DynMat _returnvalue))
  (Rendering|Material|SetMaterial (Variables|Default|GetHISM_00) 0 _output_get)
  (Utilities|Array|Clear (Variables|Default|GetColor))
  (if (> (Variables|Default|GetStones) 0)
    (for _index (range 0 (- (Variables|Default|GetStones) 1))
      (LocalVariables|SetL_Index _index)
      (Utilities|Array|Add (Variables|Default|GetColor) "(R=0.002428,G=0.138432,B=0.577581,A=1.000000)")
      (LocalVariables|SetL_StoneXLocation (+ (Spline|GetLocationatDistanceAlongSpline (Variables|Default|GetSpline) (* (LocalVariables|GetL_Index) (/ (Spline|GetSplineLength (Variables|Default|GetSpline)) (- (Variables|Default|GetStones) 1))) "World") (Math|Vector|MakeVector 0.0 0.0 (Variables|Default|GetStoneZOffset))))
      (LocalVariables|SetL_StoneXRotation (Spline|GetRotationatDistanceAlongSpline (Variables|Default|GetSpline) (* (LocalVariables|GetL_Index) (/ (Spline|GetSplineLength (Variables|Default|GetSpline)) (- (Variables|Default|GetStones) 1))) "World"))
      (bind _returnvalue_2 (Components|InstancedStaticMesh|AddInstance (Variables|Default|GetHISM_00) (Math|Transform|MakeTransform (LocalVariables|GetL_StoneXLocation) (LocalVariables|GetL_StoneXRotation)) true))
      (bind _returnvalue_3 (Rendering|Material|GetVectorParameterValue (LocalVariables|GetL_DynMat) "BaseColor" :!class /Script/Engine.MaterialInstanceDynamic))
      (Utilities|Array|SetArrayElem (Variables|Default|GetColor) (LocalVariables|GetL_Index) (select (Utilities|Array|IsValidIndex (Variables|Default|GetCustomColors) (LocalVariables|GetL_Index)) (select (!= (Math|Vector|VectorLength (Math|Conversions|ToVector(LinearColor) (Utilities|Array|Get(acopy) (Variables|Default|GetCustomColors) (LocalVariables|GetL_Index)))) 0.0) (Utilities|Array|Get(acopy) (Variables|Default|GetCustomColors) (LocalVariables|GetL_Index)) _returnvalue_3) _returnvalue_3) true)
      (Components|InstancedStaticMesh|SetCustomDataValue (Variables|Default|GetHISM_00) _returnvalue_2 0 (.R (Utilities|Struct|BreakLinearColor (Utilities|Array|Get(acopy) (Variables|Default|GetColor) (LocalVariables|GetL_Index)))) false)
      (Components|InstancedStaticMesh|SetCustomDataValue (Variables|Default|GetHISM_00) _returnvalue_2 1 (.G (Utilities|Struct|BreakLinearColor (Utilities|Array|Get(acopy) (Variables|Default|GetColor) (LocalVariables|GetL_Index)))) false)
      (Components|InstancedStaticMesh|SetCustomDataValue (Variables|Default|GetHISM_00) _returnvalue_2 2 (.B (Utilities|Struct|BreakLinearColor (Utilities|Array|Get(acopy) (Variables|Default|GetColor) (LocalVariables|GetL_Index)))) false))
    (Rendering|SetVisibility (Variables|Default|GetCubeCount) (Variables|Default|GetRenderText_?) false)
    (Rendering|SetVisibility (Variables|Default|GetBp_Name) (Variables|Default|GetRenderText_?) false)
    ;[1 1 0 0.15] Debug Only
    (if (Variables|Default|GetRenderText_?)
      (Rendering|Components|TextRender|SetText (Variables|Default|GetCubeCount) (Utilities|Text|ToText(String) (Utilities|String|Append "Cube Count : " (Utilities|String|ToString(Integer) (Components|InstancedStaticMesh|GetInstanceCount (Variables|Default|GetHISM_00)))))))))