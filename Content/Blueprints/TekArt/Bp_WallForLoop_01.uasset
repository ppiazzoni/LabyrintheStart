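; Wall Blueprint that builds a grid of stone instances and varies their depth at random when play begins.
; The construction script fills a HISM using nested loops, spacing stones along X and Z by the mesh bounds.
; BeginPlay gives each instance a random Y scale, optionally offsetting it by half its scaled depth to align stones.
; An optional debug text shows the instance count.
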(event EventBeginPlay
  (bind _sm_stone (Variables|Default|GetSM_Stone))
  (bind _returnvalue (StaticMesh|GetBoundingBox _sm_stone))
  ;[0 1 0] Begin Play
  (Variables|Default|SetStoneSizeY (.y (- (.max _returnvalue) (.min _returnvalue))))
  (if (> (Components|InstancedStaticMesh|GetInstanceCount (Variables|Default|GetHISM_00)) 0)
    (for _index (range 0 (- (Components|InstancedStaticMesh|GetInstanceCount (Variables|Default|GetHISM_00)) 1))
      (Variables|Default|SetIndex _index)
      (Variables|Default|SetRNDScaleValue (Math|Random|RandomFloatinRange (Variables|Default|GetMinScale) (Variables|Default|GetMaxScale)))
      (Components|InstancedStaticMesh|UpdateInstanceTransform (Variables|Default|GetHISM_00) (Variables|Default|GetIndex) (Math|Transform|MakeTransform (+ (.Location (Math|Transform|BreakTransform (.OutInstanceTransform (Components|InstancedStaticMesh|GetInstanceTransform (Variables|Default|GetHISM_00) (Variables|Default|GetIndex) false)))) (Math|Vector|MakeVector 0.0 (select (Variables|Default|GetAlignStones?) (* (/ (Variables|Default|GetStoneSizeY) 2.0) (Variables|Default|GetRNDScaleValue)) 0.0) 0.0)) (.Rotation (Math|Transform|BreakTransform (.OutInstanceTransform (Components|InstancedStaticMesh|GetInstanceTransform (Variables|Default|GetHISM_00) (Variables|Default|GetIndex) false)))) (Math|Vector|MakeVector 1.0 (Variables|Default|GetRNDScaleValue) 1.0)) false false false))))

(fn ConstructionScript
  (bind _sm_stone (Variables|Default|GetSM_Stone))
  (bind _sm_stone_2 (Variables|Default|GetSM_Stone))
  (bind _returnvalue (StaticMesh|GetBoundingBox _sm_stone_2))
  (bind _returnvalue_2 (StaticMesh|GetBoundingBox _sm_stone))
  (Utilities|Array|Clear (Variables|Actor|GetTags))
  (Utilities|Array|AddUnique (Variables|Actor|GetTags) "Wall_ForLoop")
  (Components|InstancedStaticMesh|ClearInstances (Variables|Default|GetHISM_00))
  (Components|StaticMesh|SetStaticMesh (Variables|Default|GetHISM_00) (Variables|Default|GetSM_Stone))
  (if (and (> (Variables|Default|GetStones_X) 0) (> (Variables|Default|GetStones_Y) 0))
    (for _index (range 0 (- (Variables|Default|GetStones_X) 1))
      (LocalVariables|SetL_StoneLocation_X (+ (* _index (Math|Vector|MakeVector (.x (- (.max _returnvalue_2) (.min _returnvalue_2))) 0.0 0.0)) (Math|Vector|MakeVector 0.0 0.0 (Variables|Default|GetStoneZOffset))))
      (for _index_2 (range 0 (- (Variables|Default|GetStones_Y) 1))
        (LocalVariables|SetL_StoneLocation_Y (* _index_2 (Math|Vector|MakeVector 0.0 0.0 (.z (- (.max _returnvalue) (.min _returnvalue))))))
        (Components|InstancedStaticMesh|AddInstance (Variables|Default|GetHISM_00) (Math|Transform|MakeTransform (+ (LocalVariables|GetL_StoneLocation_Y) (LocalVariables|GetL_StoneLocation_X))) false)))
    (Rendering|SetVisibility (Variables|Default|GetCubeCount) (Variables|Default|GetRenderText_?) false)
    (Rendering|SetVisibility (Variables|Default|GetBp_Name) (Variables|Default|GetRenderText_?) false)
    ;[1 1 0 0.15] Debug Only
    (if (Variables|Default|GetRenderText_?)
      (Rendering|Components|TextRender|SetText (Variables|Default|GetCubeCount) (Utilities|Text|ToText(String) (Utilities|String|Append "Cube Count : " (Utilities|String|ToString(Integer) (Components|InstancedStaticMesh|GetInstanceCount (Variables|Default|GetHISM_00)))))))))