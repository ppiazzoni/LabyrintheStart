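; Timed laser trap that teleports overlapping Player-tagged actors to just above a checkpoint.
; Construction stretches a capsule between two laser bases and gives both spheres a shared dynamic emissive material.
; When active, a timeline plays forward and backward after a fixed or random start delay, blending sphere colors as a FlipFlop toggles the capsule's collision and visibility.
; A DoOnce gates the teleport until the player's end overlap resets it.
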(event OnComponentBeginOverlap(Capsule)
  (params (OverlappedComponent :type Primitive%20Component%20Object%20Reference) (OtherActor :type Actor%20Object%20Reference) (OtherComp :type Primitive%20Component%20Object%20Reference) (OtherBodyIndex :type Integer) (bFromSweep :type Boolean) (SweepResult :type Hit%20Result%20Structure%20%28by%20ref%29))
  (bind _checkpoint (Variables|Default|GetCheckPoint))
  (bind _returnvalue (Transformation|GetActorTransform _checkpoint))
  (if (Actor|ActorHasTag OtherActor "Player")
    (Variables|Default|SetOther%20Actor OtherActor)
    (Utilities|FlowControl|DoOnce false
      (:Completed
        (Utilities|IsValid (Variables|Default|GetCheckPoint)
          (:Is%20Valid
            (Transformation|SetActorLocationAndRotation (Variables|Default|GetOther%20Actor) (+ (.location _returnvalue) "0.000000,0.000000,200.000000") (.rotation _returnvalue))))))))

(event OnComponentEndOverlap(Capsule)
  (params (OverlappedComponent :type Primitive%20Component%20Object%20Reference) (OtherActor :type Actor%20Object%20Reference) (OtherComp :type Primitive%20Component%20Object%20Reference) (OtherBodyIndex :type Integer))
  (if (Actor|ActorHasTag OtherActor "Player")
    (CallFunction|RDOTeleport)))

(event Custom|ReverseTimeline
  (bind _alpha (Timeline|Timeline ReverseFromEnd)
    (:Update
      (Rendering|Material|SetVectorParameterValue (Variables|Default|GetDynMat_Spheres) "EmissiveColor" (Math|Color|Lerp(LinearColor) (Variables|Default|GetSafeColor) (Variables|Default|GetColor) _alpha) :!class /Script/Engine.MaterialInstanceDynamic))
    (:Finished
      (Utilities|FlowControl|FlipFlop
        (:A
          (Collision|SetCollisionEnabled (Variables|Default|GetCapsule) "QueryOnly")
          (Rendering|SetVisibility (Variables|Default|GetCapsule) true false)
          (Rendering|Material|SetVectorParameterValue (Variables|Default|GetDynMat_Spheres) "EmissiveColor" (Variables|Default|GetDangerColor) :!class /Script/Engine.MaterialInstanceDynamic)
          (Variables|Default|SetColor (Variables|Default|GetDangerColor))
          (Utilities|FlowControl|Delay (Variables|Default|GetTrapDelay))
          (CallFunction|ReverseTimeline))
        (:B
          (Collision|SetCollisionEnabled (Variables|Default|GetCapsule) "NoCollision")
          (Rendering|SetVisibility (Variables|Default|GetCapsule) false false)
          (Rendering|Material|SetVectorParameterValue (Variables|Default|GetDynMat_Spheres) "EmissiveColor" (Variables|Default|GetSafeColor) :!class /Script/Engine.MaterialInstanceDynamic)
          (Variables|Default|SetColor (Variables|Default|GetChargeColor))
          (Utilities|FlowControl|Delay (Variables|Default|GetTrapDelay))
          (CallFunction|PlayTimeline))))))

(event Custom|PlayTimeline
  (bind _alpha (Timeline|Timeline PlayFromStart)
    (:Update
      (Rendering|Material|SetVectorParameterValue (Variables|Default|GetDynMat_Spheres) "EmissiveColor" (Math|Color|Lerp(LinearColor) (Variables|Default|GetSafeColor) (Variables|Default|GetColor) _alpha) :!class /Script/Engine.MaterialInstanceDynamic))
    (:Finished
      (Utilities|FlowControl|FlipFlop
        (:A
          (Collision|SetCollisionEnabled (Variables|Default|GetCapsule) "QueryOnly")
          (Rendering|SetVisibility (Variables|Default|GetCapsule) true false)
          (Rendering|Material|SetVectorParameterValue (Variables|Default|GetDynMat_Spheres) "EmissiveColor" (Variables|Default|GetDangerColor) :!class /Script/Engine.MaterialInstanceDynamic)
          (Variables|Default|SetColor (Variables|Default|GetDangerColor))
          (Utilities|FlowControl|Delay (Variables|Default|GetTrapDelay))
          (CallFunction|ReverseTimeline))
        (:B
          (Collision|SetCollisionEnabled (Variables|Default|GetCapsule) "NoCollision")
          (Rendering|SetVisibility (Variables|Default|GetCapsule) false false)
          (Rendering|Material|SetVectorParameterValue (Variables|Default|GetDynMat_Spheres) "EmissiveColor" (Variables|Default|GetSafeColor) :!class /Script/Engine.MaterialInstanceDynamic)
          (Variables|Default|SetColor (Variables|Default|GetChargeColor))
          (Utilities|FlowControl|Delay (Variables|Default|GetTrapDelay))
          (CallFunction|PlayTimeline))))))

(event Custom|RDO_Teleport
  (bind _checkpoint (Variables|Default|GetCheckPoint))
  (bind _returnvalue (Transformation|GetActorTransform _checkpoint))
  (Utilities|FlowControl|DoOnce false) ; enters at Reset
)

(event EventBeginPlay
  ;[0 1 0] BeginPlay
  (if (Variables|Default|GetbIsActive)
    (Collision|SetCollisionEnabled (Variables|Default|GetCapsule) "NoCollision")
    (Rendering|SetVisibility (Variables|Default|GetCapsule) false false)
    (Utilities|FlowControl|Delay (select (Variables|Default|GetbRandomDelay?) (Math|Random|RandomFloatinRange 0.0 (Variables|Default|GetMaxRandomDelay)) (Variables|Default|GetStartDelay)))
    (Components|Timeline|SetPlayRate (Variables|Default|GetTimeline) (/ 1.0 (Variables|Default|GetTL_Trap_Rate)))
    (Utilities|FlowControl|Delay (Variables|Default|GetTrapDelay))
    (CallFunction|PlayTimeline)))

(fn ConstructionScript
  (bind _laser_a (Variables|Default|GetLaser_A))
  (bind _laser_b (Variables|Default|GetLaser_B))
  (bind _relativelocation (Variables|/Script/Engine.SceneComponent|GetRelativeLocation _laser_b))
  (bind _relativelocation_2 (Variables|/Script/Engine.SceneComponent|GetRelativeLocation _laser_a))
  (Utilities|Array|Clear (Variables|Actor|GetTags))
  (Utilities|Array|AddUnique (Variables|Actor|GetTags) "LaserTrap")
  (Utilities|FlowControl|Sequence
    (:then_0
      (Transformation|SetRelativeLocation (Variables|Default|GetLaser_B) (Variables|Default|GetLaserBase_B_Location) false false)
      (bind _output_get (LocalVariables|SetL_MidDistance (/ (- _relativelocation _relativelocation_2) 2.0)))
      (Transformation|SetRelativeLocationAndRotation (Variables|Default|GetCapsule) _output_get (Math|Rotator|CombineRotators "90.000000,0.000000,0.000000" (Math|Rotator|FindLookatRotation _relativelocation _relativelocation_2)) false false)
      (Components|Capsule|SetCapsuleHalfHeight (Variables|Default|GetCapsule) (Math|Vector|VectorLength (LocalVariables|GetL_MidDistance)) true)
      (Components|Capsule|SetCapsuleRadius (Variables|Default|GetCapsule) (Variables|Default|GetCapsuleRadius) true))
    (:then_1
      (bind _returnvalue (Rendering|Material|CreateDynamicMaterialInstance (Variables|Default|GetSphere_B) 0 "/Game/Blueprints/Materials/MI_Basic_Green.MI_Basic_Green" "None" :!class /Script/Engine.PrimitiveComponent))
      (bind _output_get_2 (Variables|Default|SetDynMat_Spheres _returnvalue))
      (Rendering|Material|SetMaterial (Variables|Default|GetSphere_A) 0 _output_get_2)
      (Rendering|Material|SetVectorParameterValue (Variables|Default|GetDynMat_Spheres) "EmissiveColor" (Variables|Default|GetSafeColor) :!class /Script/Engine.MaterialInstanceDynamic)
      (Variables|Default|SetColor (Variables|Default|GetChargeColor)))))