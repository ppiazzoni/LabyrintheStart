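; Laser trap that sends an overlapping player to just above its checkpoint.
; A timeline, started after an optional random delay when active, ping-pongs the laser A pivot to a destination with pauses at each end.
; The construction script fits the hit capsule between both laser pivots and tints the end spheres through a shared dynamic material.
; A DoOnce gates the teleport until the player leaves the capsule.
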(event OnComponentBeginOverlap(Capsule)
  (params (OverlappedComponent :type Primitive%20Component%20Object%20Reference) (OtherActor :type Actor%20Object%20Reference) (OtherComp :type Primitive%20Component%20Object%20Reference) (OtherBodyIndex :type Integer) (bFromSweep :type Boolean) (SweepResult :type Hit%20Result%20Structure%20%28by%20ref%29))
  (bind _checkpoint (Variables|Default|GetCheckPoint))
  (bind _returnvalue (Transformation|GetActorTransform _checkpoint))
  (if (Actor|ActorHasTag OtherActor "Player")
    (Variables|Default|SetOther%20Actor OtherActor)
    (Utilities|FlowControl|DoOnce false
      (:Completed
        (Utilities|IsValid (Variables|Default|GetCheckPoint)
          (:Is%20Valid
            (Transformation|SetActorLocationAndRotation (+ (.location _returnvalue) "0.000000,0.000000,200.000000") (.rotation _returnvalue))))))))

(event OnComponentEndOverlap(Capsule)
  (params (OverlappedComponent :type Primitive%20Component%20Object%20Reference) (OtherActor :type Actor%20Object%20Reference) (OtherComp :type Primitive%20Component%20Object%20Reference) (OtherBodyIndex :type Integer))
  (if (Actor|ActorHasTag OtherActor "Player")
    (CallFunction|RDOTeleport)))

(event Custom|ReverseTimeline
  (bind _alpha (Timeline|Timeline ReverseFromEnd)
    (:Update
      (Variables|Default|SetAlpha _alpha)
      (Transformation|SetRelativeLocation (Variables|Default|GetLaserA_Pivot) (Math|Vector|Lerp(Vector) "0, 0, 0" (Variables|Default|GetDestination_Location) (Variables|Default|GetAlpha)) false false))
    (:Finished
      (Utilities|FlowControl|FlipFlop
        (:A
          (Utilities|FlowControl|Delay (Variables|Default|GetTrapDelay))
          (CallFunction|ReverseTimeline))
        (:B
          (Utilities|FlowControl|Delay (Variables|Default|GetTrapDelay))
          (CallFunction|PlayTimeline))))))

(event Custom|PlayTimeline
  (bind _alpha (Timeline|Timeline PlayFromStart)
    (:Update
      (Variables|Default|SetAlpha _alpha)
      (Transformation|SetRelativeLocation (Variables|Default|GetLaserA_Pivot) (Math|Vector|Lerp(Vector) "0, 0, 0" (Variables|Default|GetDestination_Location) (Variables|Default|GetAlpha)) false false))
    (:Finished
      (Utilities|FlowControl|FlipFlop
        (:A
          (Utilities|FlowControl|Delay (Variables|Default|GetTrapDelay))
          (CallFunction|ReverseTimeline))
        (:B
          (Utilities|FlowControl|Delay (Variables|Default|GetTrapDelay))
          (CallFunction|PlayTimeline))))))

(event Custom|RDO_Teleport
  (bind _checkpoint (Variables|Default|GetCheckPoint))
  (bind _returnvalue (Transformation|GetActorTransform _checkpoint))
  (Utilities|FlowControl|DoOnce false) ; enters at Reset
)

(event EventBeginPlay
  ;[0 1 0] BeginPlay
  (if (Variables|Default|GetbIsActive)
    (Utilities|FlowControl|Delay (select (Variables|Default|GetbRandomDelay?) (Math|Random|RandomFloatinRange 0.0 (Variables|Default|GetMaxRandomDelay)) (Variables|Default|GetStartDelay)))
    (Components|Timeline|SetPlayRate (Variables|Default|GetTimeline) (/ 1.0 (Variables|Default|GetTL_Trap_Rate)))
    (Utilities|FlowControl|Delay (Variables|Default|GetTrapDelay))
    (CallFunction|PlayTimeline)))

(fn ConstructionScript
  (bind _lasera_pivot (Variables|Default|GetLaserA_Pivot))
  (bind _laserb_pivot (Variables|Default|GetLaserB_Pivot))
  (bind _relativelocation (Variables|/Script/Engine.SceneComponent|GetRelativeLocation _laserb_pivot))
  (bind _relativelocation_2 (Variables|/Script/Engine.SceneComponent|GetRelativeLocation _lasera_pivot))
  (Utilities|Array|Clear (Variables|Actor|GetTags))
  (Utilities|Array|AddUnique (Variables|Actor|GetTags) "LaserTrap")
  (Utilities|FlowControl|Sequence
    (:then_0
      (Transformation|SetRelativeLocation (Variables|Default|GetLaserB_Pivot) (Variables|Default|GetLaserBase_B_Location) false false)
      (bind _output_get (LocalVariables|SetL_MidDistance (/ (- _relativelocation _relativelocation_2) 2.0)))
      (Transformation|SetRelativeLocationAndRotation (Variables|Default|GetCapsule) _output_get (Math|Rotator|CombineRotators "90.000000,0.000000,0.000000" (Math|Rotator|FindLookatRotation _relativelocation _relativelocation_2)) false false)
      (Components|Capsule|SetCapsuleHalfHeight (Variables|Default|GetCapsule) (Math|Vector|VectorLength (LocalVariables|GetL_MidDistance)) true)
      (Components|Capsule|SetCapsuleRadius (Variables|Default|GetCapsule) (Variables|Default|GetCapsuleRadius) true)
      (Transformation|SetRelativeLocation (Variables|Default|GetDestination_Pivot) (Variables|Default|GetDestination_Location) false false))
    (:then_1
      (bind _returnvalue (Rendering|Material|CreateDynamicMaterialInstance (Variables|Default|GetSphere_B) 0 0 "None" :!class /Script/Engine.PrimitiveComponent))
      (bind _output_get_2 (Variables|Default|SetDynMat_Spheres _returnvalue))
      (Rendering|Material|SetMaterial (Variables|Default|GetSphere_A) 0 _output_get_2)
      (Rendering|Material|SetVectorParameterValue (Variables|Default|GetDynMat_Spheres) "EmissiveColor" (Variables|Default|GetSafeColor) :!class /Script/Engine.MaterialInstanceDynamic)
      (Variables|Default|SetColor (Variables|Default|GetChargeColor)))))